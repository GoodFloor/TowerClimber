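; BP_PlatformerChar is a 2D sprite platformer character Blueprint that handles the character's defeat.
; Its Defeat event runs once, disabling capsule collision, releasing the movement plane constraint and launching the character along combined up and right vectors scaled by variables.
; It then jumps the animation instance to the defeated node and raises the sprite's translucency sort priority so it can draw over other translucent objects.
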(event `Defeat`
  (if (not (`self.IsDefeated`))
    (set `self.IsDefeated` true)
    (`PrimitiveComponent.SetCollisionEnabled` (`self.CapsuleComponent`) "NoCollision")
    (`MovementComponent.SetPlaneConstraintEnabled` (`self.CharacterMovement`) false)
    (`self.LaunchOnDefeat`)
    (`PaperZDAnimInstance.JumpToNode` (`self.GetAnimInstance`) "JumpDefeated" "None")
    (`PrimitiveComponent.SetTranslucentSortPriority` (`self.Sprite`) 100)))

(fn `LaunchOnDefeat`
  (`self.LaunchCharacter` (+ (* (`KismetMathLibrary.Vector_Up`) (`self.DefeatUpLaunch`)) (* (`KismetMathLibrary.Vector_Right`) (`self.DefeatForwardLaunch`))) true true))

(fn `UserConstructionScript`)